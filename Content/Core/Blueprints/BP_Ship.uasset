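; BP_Ship is the player ship Blueprint, handling HUD setup and mouse-to-world projection.
; On BeginPlay it clears existing widgets and creates WBP_HUD for the local player, then assigns itself as owner of its WBP_HealthBar widget component.
; GetMouseLocationOnYZ intersects the deprojected cursor ray with the X=0 plane, returning zero when no intersection is possible.
; Tick is empty, and the weapon and movement debug nodes are unconnected.
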(event `self.ReceiveTick`
  (params (DeltaSeconds :type "Float (single-precision)")))

(event `self.ReceiveBeginPlay`
  (`self.InitPlayerHUD`)
  (`self.InitHealthBarWidget`))

(fn `GetMouseLocationOnYZ`
  (returns (ProjectedMouseLocation :type "Vector Structure"))
  (bind _asplayer_controller (cast `PlayerController` (`self.GetController`))
    (:`then`
      (bind (_worldlocation _worlddirection) (`PlayerController.DeprojectMousePositionToWorld` _asplayer_controller))
      (bind _x (.x _worlddirection))
      (if (!= _x 0.0)
        (return (+ (* (/ (- 0.0 (.x _worldlocation)) _x) _worlddirection) _worldlocation))
        (else
          _)))
    (:`CastFailed`
      _))
  (return (0.0 0.0 0.0)))

(fn `InitHealthBarWidget`
  (bind _aswbp_health_bar (cast `/Game/Core/UI/WBP_HealthBar` (`WidgetComponent.GetWidget` (`self.HealthBarWidget`))))
  (set `/Game/Core/UI/WBP_HealthBar.OwnerPawn` self _aswbp_health_bar))

(fn `InitPlayerHUD`
  (bind _returnvalue (`GameplayStatics.GetPlayerController` 0))
  (`/Engine/EditorBlueprintResources/StandardMacros.IsValid` _returnvalue
    (:`Is Valid`
      (if (`Controller.IsLocalPlayerController` _returnvalue)
        (`WidgetLayoutLibrary.RemoveAllWidgets`)
        (bind _returnvalue_2 (`|CreateWidget` "/Game/Core/UI/WBP_HUD.WBP_HUD_C"))
        (`UserWidget.AddToViewport` _returnvalue_2 0)))))

(fn `UserConstructionScript`)