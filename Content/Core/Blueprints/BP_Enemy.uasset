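; BP_Enemy is an enemy Blueprint with a health bar widget and an on-screen state readout.
; On BeginPlay it casts the HealthBarWidget component's widget to WBP_HealthBar and sets itself as that widget's OwnerPawn.
; Tick prints the current enemy state every frame as debug output.
; An unconnected StopMovementImmediately call on the movement component never runs.
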(event `self.ReceiveBeginPlay`
  (`self.InitHealthBarWidget`))

(event `self.ReceiveTick`
  (params (DeltaSeconds :type "Float (single-precision)"))
  (`KismetSystemLibrary.PrintString` (`|GetEnumeratorNameAsString` (`self.GetEnemyState`)) true true (struct :`G` 0.66 :`B` 1.0 :`A` 1.0) 0.0))

(fn `InitHealthBarWidget`
  (bind _aswbp_health_bar (cast `/Game/Core/UI/WBP_HealthBar` (`WidgetComponent.GetWidget` (`self.HealthBarWidget`))))
  (set `/Game/Core/UI/WBP_HealthBar.OwnerPawn` self _aswbp_health_bar))

(fn `UserConstructionScript`)